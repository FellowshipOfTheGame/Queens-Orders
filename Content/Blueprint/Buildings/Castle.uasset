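; Castle building Blueprint that exposes child-actor building spots through an interface.
; GetSpots casts the Spot1 and Spot2 child actors to the building spot interface in a sequence and returns both references; Spot3 is not included.
; If Spot1 fails the first interface cast, it prints a Portuguese error and quits the game.
; Cursor-over and click events on Spot3 and Box1 only print debug strings.
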(event `self.Spot3.OnBeginCursorOver`
  (params (TouchedComponent :type "PrimitiveComponent Object Reference"))
  (`KismetSystemLibrary.PrintString` "spot3OVER"))

(event `self.Box1.OnClicked`
  (params (TouchedComponent :type "PrimitiveComponent Object Reference"))
  (`KismetSystemLibrary.PrintString` "Hello"))

(event `self.Spot3.OnClicked`
  (params (TouchedComponent :type "PrimitiveComponent Object Reference"))
  (`KismetSystemLibrary.PrintString` "Click on box"))

(fn `GetSpots`
  (returns (spots :type "Array of /Game/Blueprints/Buildings/IBuildingSpot Interface"))
  (`|ExecutionSequence`
    (:`then_0`
      (bind _asinterface (cast `Interface` (`ChildActorComponent.ChildActor` (`self.Spot1`)))
        (:`then`
          (bind _asibuildingspot_c (cast `/Game/Blueprints/Buildings/IBuildingSpot` _asinterface)))
        (:`CastFailed`
          (`KismetSystemLibrary.PrintString` "OPS! Objeto nao eh da interface correta!")
          (`KismetSystemLibrary.QuitGame` null "Quit")
          (return (`|MakeArray` _asibuildingspot_c (stale _asibuildingspot_c_2))))))
    (:`then_1`
      (bind _asinterface_2 (cast `Interface` (`ChildActorComponent.ChildActor` (`self.Spot2`))))
      (bind _asibuildingspot_c_2 (cast `/Game/Blueprints/Buildings/IBuildingSpot` _asinterface_2)))
    (:`then_5`
      (return (`|MakeArray` _asibuildingspot_c _asibuildingspot_c_2)))))

(fn `UserConstructionScript`)