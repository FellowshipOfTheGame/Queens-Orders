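; Base building Blueprint that tracks health and whether construction or repair is complete.
; SetHealth stores the new value and, when it exceeds GetMaxHealth, clamps it, then either marks the building built or reports a repair, printing a message.
; The construction script starts it unbuilt at zero health.
; GetMaxHealth returns zero and StartBuilding and FinishBuilding are empty stubs, while GetHealth and IsBuilt expose state.
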(event `self.Set Health`
  (params (life :type "Float (single-precision)"))
  ;[1 1 1] Set Health
  (set `self.health` life)
  (bind _maxhealth (`self.Get Max Health`))
  (if (> (`self.health`) _maxhealth)
    ;[1 1 1] Finish Building - Set Max Health and FeedBack
    (set `self.health` _maxhealth)
    (if (`self.built`)
      (`KismetSystemLibrary.PrintString` "Repair complete!")
      (else
        (set `self.built` true)
        (`KismetSystemLibrary.PrintString` "Building Complete!")))))

(fn `Finish Building`)

(fn `Get Health`
  (returns (life :type "Float (double-precision)"))
  (return (`self.health`)))

(fn `Get Max Health`
  (returns (MaxHealth :type "Float (double-precision)"))
  (return 0.0))

(fn `IsBuilt`
  (returns (built :type Boolean))
  (return (`self.built`)))

(fn `StartBuilding`)

(fn `UserConstructionScript`
  (set `self.health` 0.0)
  (set `self.built` false))