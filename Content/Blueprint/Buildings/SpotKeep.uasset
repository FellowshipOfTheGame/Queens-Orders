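; SpotKeep is a building spot Blueprint for the Keep that players can click.
; Clicking its CollisionArea sets it as the CurrentBuildingSpot on MyController, then prints a placeholder message for the Keep options UI.
; GetBuildingType returns a fixed enum value, while GetCurrentBuilding returns no set building and OnBuildOnSpot always returns false, so this spot accepts no construction.
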(event `self.CollisionArea.OnClicked`
  (params (TouchedComponent :type "PrimitiveComponent Object Reference"))
  (bind _asmycontroller_c (cast `/Game/Blueprints/MyController` (`GameplayStatics.GetPlayerController` 0)))
  (set `/Game/Blueprints/MyController.currentBuildingSpot` self _asmycontroller_c)
  (`KismetSystemLibrary.PrintString` "Show UI for Keeps options"))

(fn `getBuildingType`
  (returns (type :type "/Game/Blueprints/Buildings/BuildingSpotTypes Enum"))
  (return "NewEnumerator3"))

(fn `GetCurrentBuilding`
  (returns (building :type "/Game/Blueprints/Buildings/Building Object Reference"))
  (return null))

(fn `OnBuildOnSpot`
  (params (BuildingObject :type "/Game/Blueprints/Buildings/BuildingTypes Enum" :default "NewEnumerator0"))
  (returns (state :type Boolean))
  (return false))

(fn `UserConstructionScript`)