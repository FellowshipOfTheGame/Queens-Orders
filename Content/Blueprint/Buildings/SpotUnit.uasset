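; SpotUnit is a clickable building spot for unit buildings, offering Barracks and Ranger as build options.
; A click registers it as the controller's current building spot and opens the on-screen build menu through MyHUD.
; OnBuildOnSpot refuses if already occupied; otherwise it spawns the chosen building, attaches it to the spot and starts construction.
; Getters expose the spot's type and current building.
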(event OnClicked(Collision)
  (params (TouchedComponent :type Primitive%20Component%20Object%20Reference))
  (bind _asmycontroller_c (Utilities|Casting|CastToMyController (Game|GetPlayerController 0)))
  (Variables|/Game/Blueprints/MyController.MyController_C|SetcurrentBuildingSpot _asmycontroller_c self)
  (Development|PrintString "Show UI for UnitBuilds options [barracks, ranger, etc]")
  (bind _asmyhud_c (Utilities|Casting|CastToMyHUD (HUD|GetHUD _asmycontroller_c)))
  (Default|OpenonScreenBuildOptions _asmyhud_c (Variables|Default|Getbuildoptions)))

(fn ConstructionScript
  (Variables|Default|Setbuildoptions (Utilities|Array|MakeArray "NewEnumerator0" "NewEnumerator1")))

(fn GetBuildingType
  (return "NewEnumerator1"))

(fn GetCurrentBuilding
  (return (Variables|Default|GetCurrentBuilding)))

(fn OnBuildonSpot
  (params (BuildingObject :type BuildingTypes%20Enum :default "NewEnumerator0"))
  (bind _returnvalue (Transformation|GetActorTransform))
  (bind (_location _rotation _scale) (Math|Transform|BreakTransform _returnvalue))
  (bind _returnvalue_2 (Math|Transform|MakeTransform "0.000000,0.000000,0.000000" _rotation _scale))
  (if (Utilities|IsValid (Variables|Default|GetCurrentBuilding))
    (LocalVariables|Settmp1 false)
    (else
      (LocalVariables|Settmp1 true)
      (switch Utilities|FlowControl|Switch|SwitchonBuildingTypes BuildingObject
        (:NewEnumerator0
          (bind _returnvalue_3 (Game|SpawnActorfromClass "/Game/Blueprints/Buildings/Barracks.Barracks_C" _returnvalue_2 false 0))
          (Variables|Default|SetCurrentBuilding _returnvalue_3))
        (:NewEnumerator1
          (bind _returnvalue_4 (Game|SpawnActorfromClass "/Game/Blueprints/Buildings/Ranger.Ranger_C" _returnvalue_2 false 0))
          (Variables|Default|SetCurrentBuilding _returnvalue_4)))
      (Class|Actor|AttachRootComponenttoActor (Variables|Default|GetCurrentBuilding) self "None" "KeepRelativeOffset" true)
      (Default|StartBuilding (Variables|Default|GetCurrentBuilding))))
  (return (LocalVariables|Gettmp1)))