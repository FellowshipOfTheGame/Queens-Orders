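; HUD Blueprint that draws a green box-selection rectangle on screen while Pressing is true.
; Each DrawHUD call draws four lines between the stored XPosition/YPosition corner and the current mouse position.
; It only handles the visual: nothing here sets the flag or corner, or selects objects.
; A DrawBox node is present but never runs.
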(event `self.ReceiveDrawHUD`
  (params (SizeX :type Integer) (SizeY :type Integer))
  (bind _returnvalue (`GameplayStatics.GetPlayerController` 0))
  (bind _xposition (`self.xPosition`))
  (bind _yposition (`self.yPosition`))
  (bind (_locationx _locationy) (`PlayerController.GetMousePosition` _returnvalue))
  (bind _returnvalue_2 (`PlayerController.GetHUD` _returnvalue))
  (if (`self.pressing`)
    (`|ExecutionSequence`
      (:`then_0`
        (`self.DrawLine` _returnvalue_2 _xposition _yposition _locationx _yposition (struct :`G` 1.0 :`A` 1.0)))
      (:`then_1`
        (`self.DrawLine` _returnvalue_2 _xposition _yposition _xposition _locationy (struct :`G` 1.0 :`A` 1.0)))
      (:`then_2`
        (`self.DrawLine` _returnvalue_2 _xposition _locationy _locationx _locationy (struct :`G` 1.0 :`A` 1.0)))
      (:`then_3`
        (`self.DrawLine` _returnvalue_2 _locationx _yposition _locationx _locationy (struct :`G` 1.0 :`A` 1.0))))))

(fn `UserConstructionScript`)