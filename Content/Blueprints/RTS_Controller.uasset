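; RTS controller Blueprint that handles mouse box selection, building slot selection and building deletion.
; Left mouse press and release set the pressed state on RTS_HUD, with the press also recording the cursor position as the box origin.
; SetCurrentBuildingSlot hides the previous slot's options, stores the new slot and shows its options.
; Delete destroys the building that the current slot returns through a message call.
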(event `Key|LeftMouseButton`
  (bind _returnvalue (`GameplayStatics.GetPlayerController` 0))
  (bind (_locationx _locationy) (`self.GetMousePosition` _returnvalue))
  (bind _returnvalue_2 (`self.GetHUD` _returnvalue))
  ;[1 1 1] BoxSelection
  (:`Pressed`
    (bind _asrts_hud_c (cast `/Game/Blueprints/RTS_HUD` _returnvalue_2))
    (set `/Game/Blueprints/RTS_HUD.pressing` true _asrts_hud_c)
    (set `/Game/Blueprints/RTS_HUD.xPosition` _locationx _asrts_hud_c)
    (set `/Game/Blueprints/RTS_HUD.yPosition` _locationy _asrts_hud_c))
  (:`Released`
    (bind _asrts_hud_c_2 (cast `/Game/Blueprints/RTS_HUD` _returnvalue_2))
    (set `/Game/Blueprints/RTS_HUD.pressing` false _asrts_hud_c_2)))

(event `Key|Delete`
  (bind _currentbuildingslot (`self.currentBuildingSlot`))
  ;[1 1 1] Destruir construcao
  (:`Pressed`
    (`/Engine/EditorBlueprintResources/StandardMacros.IsValid` _currentbuildingslot
      (:`Is Valid`
        (bind _building (message `/Game/Blueprints/Buildings/BuildingSlots/IBuildingSlot.GetBuiltBuilding` _currentbuildingslot))
        (`self.K2_DestroyActor` _building)))))

(fn `Set Current Building Slot`
  (params (spot :type "/Game/Blueprints/Buildings/BuildingSlots/BuildingSlot Object Reference"))
  (bind _currentbuildingslot (`self.currentBuildingSlot`))
  ;[1 1 1] Set Current Selected Building Spot
  (`/Engine/EditorBlueprintResources/StandardMacros.IsValid` _currentbuildingslot
    (:`Is Valid`
      (`/Game/Blueprints/Buildings/BuildingSlots/BuildingSlot.HideOptions` _currentbuildingslot))
    (:`Is Not Valid`
      _))
  (set `self.currentBuildingSlot` spot)
  (`/Game/Blueprints/Buildings/BuildingSlots/BuildingSlot.ShowOptions` spot)
  (`KismetSystemLibrary.PrintString` "Selected"))

(fn `UserConstructionScript`)