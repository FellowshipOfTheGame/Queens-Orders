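; HUD that draws a building health bar and a drag-selection box on screen.
; Each DrawHUD finds the MyController's current building spot, drawing a black backing and a green fill sized directly by the building's health message.
; While Pressing is true, four green lines form a rectangle from the stored X/Y position to the mouse.
; OpenOnScreenBuildOptions is a stub that only prints a string.
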(event `self.ReceiveDrawHUD`
  (params (SizeX :type Integer) (SizeY :type Integer))
  (bind _returnvalue (`GameplayStatics.GetPlayerController` 0))
  (bind _returnvalue_2 (`GameplayStatics.GetPlayerController` 0))
  (bind _xposition (`self.xPosition`))
  (bind _yposition (`self.yPosition`))
  (bind (_locationx _locationy) (`PlayerController.GetMousePosition` _returnvalue))
  (bind _returnvalue_3 (`PlayerController.GetHUD` _returnvalue))
  (`|ExecutionSequence`
    (:`then_0`
      ;[1 1 1] Draw Health bar
      (`|ExecutionSequence`
        (:`then_1`
          (if (`KismetSystemLibrary.IsValid` _returnvalue_2)
            (bind _asmycontroller_c (cast `/Game/Blueprints/MyController` _returnvalue_2))
            (bind _currentbuildingspot (`/Game/Blueprints/MyController.currentBuildingSpot` _asmycontroller_c))
            (`/Engine/EditorBlueprintResources/StandardMacros.IsValid` _currentbuildingspot
              (:`Is Valid`
                (bind _building (`/Game/Blueprints/Buildings/IBuildingSpot.GetCurrentBuilding` _currentbuildingspot))
                (`|ExecutionSequence`
                  (:`then_0`
                    (`self.DrawRect` (struct :`A` 1.0) 0.0 0.0 200.0 32.0))
                  (:`then_1`
                    (`/Engine/EditorBlueprintResources/StandardMacros.IsValid` _building
                      (:`Is Valid`
                        (bind _life (message `/Game/Blueprints/IUnit.Get Health` _building))
                        (`self.DrawRect` (struct :`R` 0.140292 :`G` 0.705 :`B` 0.029192 :`A` 1.0) 0.0 1.0 _life 30.0)))))))))))
    (:`then_1`
      ;[1 1 1] Draw Selection Square
      (if (`self.pressing`)
        (`|ExecutionSequence`
          (:`then_0`
            (`self.DrawLine` _returnvalue_3 _xposition _yposition _locationx _yposition (struct :`G` 1.0 :`A` 1.0)))
          (:`then_1`
            (`self.DrawLine` _returnvalue_3 _xposition _yposition _xposition _locationy (struct :`G` 1.0 :`A` 1.0)))
          (:`then_2`
            (`self.DrawLine` _returnvalue_3 _xposition _locationy _locationx _locationy (struct :`G` 1.0 :`A` 1.0)))
          (:`then_3`
            (`self.DrawLine` _returnvalue_3 _locationx _yposition _locationx _locationy (struct :`G` 1.0 :`A` 1.0))))))))

(fn `openOnScreenBuildOptions`
  (params (NewParam :type "Array of /Game/Blueprints/Buildings/BuildingTypes Enum"))
  (`KismetSystemLibrary.PrintString` "Hello"))

(fn `UserConstructionScript`)