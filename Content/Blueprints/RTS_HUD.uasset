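; RTS HUD that draws a health bar for the selected building and a drag-selection box each frame.
; The bar sits at the building's projected screen position, with green width taken directly from CurrentHP over a fixed-width black backing.
; While Pressing is true, four green lines box the area from XPosition/YPosition to the mouse cursor.
; This graph only reads those drag variables and never sets them.
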(event `self.ReceiveDrawHUD`
  (params (SizeX :type Integer) (SizeY :type Integer))
  (bind _returnvalue (`GameplayStatics.GetPlayerController` 0))
  (bind _returnvalue_2 (`GameplayStatics.GetPlayerController` 0))
  (bind _xposition (`self.xPosition`))
  (bind _yposition (`self.yPosition`))
  (bind (_locationx _locationy) (`PlayerController.GetMousePosition` _returnvalue))
  (bind _returnvalue_3 (`PlayerController.GetHUD` _returnvalue))
  (`|ExecutionSequence`
    (:`then_0`
      ;[1 1 1] Draw Health bar
      (`|ExecutionSequence`
        (:`then_0`
          (bind _asrts_controller (cast `RTS_Controller` _returnvalue_2))
          (bind _returnvalue_4 (`RTS_Controller.getCurrentSelectedSlot` _asrts_controller))
          (`/Engine/EditorBlueprintResources/StandardMacros.IsValid` _returnvalue_4
            (:`Is Valid`
              (bind _building (`BuildingSlot.building` _returnvalue_4))
              (`/Engine/EditorBlueprintResources/StandardMacros.IsValid` _building
                (:`Is Valid`
                  (`|ExecutionSequence`
                    (:`then_0`
                      (bind (_x _y) (`KismetMathLibrary.BreakVector2D` (`PlayerController.ProjectWorldLocationToScreen` _returnvalue_2 (`self.K2_GetActorLocation` _building))))
                      (`self.DrawRect` (struct :`A` 1.0) _x (- _y 1.0) 200.0 32.0))
                    (:`then_1`
                      (`self.DrawRect` (struct :`R` 0.140292 :`G` 0.705 :`B` 0.029192 :`A` 1.0) _x _y (`Building.currentHP` _building) 30.0))))))))))
    (:`then_1`
      ;[1 1 1] Draw Selection Square
      (if (`self.pressing`)
        (`|ExecutionSequence`
          (:`then_0`
            (`self.DrawLine` _returnvalue_3 _xposition _yposition _locationx _yposition (struct :`G` 1.0 :`A` 1.0)))
          (:`then_1`
            (`self.DrawLine` _returnvalue_3 _xposition _yposition _xposition _locationy (struct :`G` 1.0 :`A` 1.0)))
          (:`then_2`
            (`self.DrawLine` _returnvalue_3 _xposition _locationy _locationx _locationy (struct :`G` 1.0 :`A` 1.0)))
          (:`then_3`
            (`self.DrawLine` _returnvalue_3 _locationx _yposition _locationx _locationy (struct :`G` 1.0 :`A` 1.0))))))))

(fn `UserConstructionScript`)