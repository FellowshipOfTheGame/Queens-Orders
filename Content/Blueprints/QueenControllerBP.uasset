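; Queen controller Blueprint that opens an in-world UI for a selected building slot.
; OpenUIForBuildingSlot spawns a BuildingSlotUI actor at the slot, then casts through gate, ranger barracks, tower ranger barracks and tower types to add a widget component.
; The raised, enlarged widget receives the slot reference.
; Its test camera-facing rotation is computed once, from the relative offset rather than the slot's world position.
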(fn ConstructionScript)

(fn OpenUIforBuildingSlot
  (params (slot :type Building%20Slot%20Object%20Reference))
  (bind _returnvalue (Math|Vector|MakeVector 3.0 3.0 3.0))
  (bind _returnvalue_2 (Game|GetPlayerCameraManager 0))
  (bind _returnvalue_3 (Math|Vector|MakeVector 0.0 0.0 2e+03))
  (bind _returnvalue_4 (Transformation|GetActorLocation _returnvalue_2))
  (bind _returnvalue_5 (Math|Rotator|FindLookatRotation _returnvalue_3 _returnvalue_4))
  (bind _returnvalue_6 (Math|Transform|MakeTransform _returnvalue_3 _returnvalue_5 _returnvalue))
  (bind _returnvalue_7 (Game|SpawnActorfromClass "/Game/Blueprints/Buildings/BuildingSlots/Widgets/BuildingSlotUI.BuildingSlotUI_C" (Transformation|GetActorTransform slot) false 0))
  (LocalVariables|SetnewUI _returnvalue_7)
  ;[1 1 1] Spawn Correct Widget Object
  (Utilities|Casting|CastToSlot_Gate slot
    (:then
      (bind _returnvalue_8 (AddComponent|AddWidgetComponent (LocalVariables|GetnewUI) false _returnvalue_6))
      (LocalVariables|Setwidget (UserInterface|GetUserWidgetObject _returnvalue_8)))
    (:CastFailed
      (Utilities|Casting|CastToSlot_RangerBarracks slot
        (:then
          (bind _returnvalue_9 (AddComponent|AddWidgetComponent (LocalVariables|GetnewUI) false _returnvalue_6))
          (LocalVariables|Setwidget (UserInterface|GetUserWidgetObject _returnvalue_9)))
        (:CastFailed
          (Utilities|Casting|CastToSlot_TowerRangerBarracks slot
            (:then
              (bind _returnvalue_10 (AddComponent|AddWidgetComponent (LocalVariables|GetnewUI) false _returnvalue_6))
              (LocalVariables|Setwidget (UserInterface|GetUserWidgetObject _returnvalue_10)))
            (:CastFailed
              (Utilities|Casting|CastToSlot_Tower slot)
              (bind _returnvalue_11 (AddComponent|AddWidgetComponent (LocalVariables|GetnewUI) false _returnvalue_6))
              (LocalVariables|Setwidget (UserInterface|GetUserWidgetObject _returnvalue_11))))))))
  (bind _aswidget_slot (Utilities|Casting|CastToWidgetSlot (LocalVariables|Getwidget)))
  (Variables|/Game/Blueprints/Buildings/BuildingSlots/Widgets/WidgetSlot.WidgetSlot_C|SetMySlot _aswidget_slot slot)
  (return (LocalVariables|GetnewUI)))