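; SpotUnit is a clickable RTS building spot that can host one Barracks or Ranger building.
; Clicking its collision registers it with the RTS_Controller as the current spot, and getters expose its build options, type and current building.
; OnBuildOnSpot rejects occupied spots, otherwise spawns the chosen building at zero location with the spot's rotation and scale, attaches it and calls StartBuilding.
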(event OnClicked(Collision)
  (params (TouchedComponent :type Primitive%20Component%20Object%20Reference))
  (bind _asrts_controller_c (Utilities|Casting|CastToRTS_Controller (Game|GetPlayerController 0)))
  (Default|SetCurrentBuildingSpot _asrts_controller_c self))

(fn ConstructionScript
  (Variables|Default|Setbuildoptions (Utilities|Array|MakeArray "NewEnumerator0" "NewEnumerator1")))

(fn GetBuildingPossibleTypes
  (return (Variables|Default|Getbuildoptions)))

(fn GetBuildingType
  (return "NewEnumerator1"))

(fn GetCurrentBuilding
  (return (Variables|Default|GetCurrentBuilding)))

(fn OnBuildonSpot
  (params (BuildingObject :type BuildingTypes%20Enum :default "NewEnumerator0"))
  (bind _returnvalue (Transformation|GetActorTransform))
  (bind (_location _rotation _scale) (Math|Transform|BreakTransform _returnvalue))
  (bind _returnvalue_2 (Math|Transform|MakeTransform "0.000000,0.000000,0.000000" _rotation _scale))
  (if (Utilities|IsValid (Variables|Default|GetCurrentBuilding))
    (LocalVariables|Settmp1 false)
    (else
      (LocalVariables|Settmp1 true)
      (switch Utilities|FlowControl|Switch|SwitchonBuildingTypes BuildingObject
        (:NewEnumerator0
          (bind _returnvalue_3 (Game|SpawnActorfromClass "/Game/Blueprints/Buildings/Barracks.Barracks_C" _returnvalue_2 false 0))
          (Variables|Default|SetCurrentBuilding _returnvalue_3))
        (:NewEnumerator1
          (bind _returnvalue_4 (Game|SpawnActorfromClass "/Game/Blueprints/Buildings/Ranger.Ranger_C" _returnvalue_2 false 0))
          (Variables|Default|SetCurrentBuilding _returnvalue_4)))
      (Class|Actor|AttachRootComponenttoActor (Variables|Default|GetCurrentBuilding) self "None" "KeepRelativeOffset" true)
      (Default|StartBuilding (Variables|Default|GetCurrentBuilding))))
  (return (LocalVariables|Gettmp1)))