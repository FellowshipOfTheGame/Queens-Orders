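; Ranger building Blueprint that reports its building type and maximum health and handles its own construction progress.
; While it is not built, each Tick adds a fixed amount to Health, independent of delta time.
; It then shows the Collision component and its children only when Health exactly equals the maximum, hiding them otherwise.
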(event `self.ReceiveTick`
  (params (DeltaSeconds :type "Float (single-precision)"))
  (bind _collision (`self.Collision`))
  (bind _built (message `/Game/Blueprints/IUnit.IsBuilt` self))
  (if (not _built)
    (`self.Set Health` (+ (`self.health`) 1.0))
    (bind _maxhealth (message `/Game/Blueprints/IUnit.Get Max Health` self))
    (if (== _maxhealth (`self.health`))
      (`SceneComponent.SetVisibility` _collision true true)
      (else
        (`SceneComponent.SetVisibility` _collision false true)))))

(fn `Get Max Health`
  (returns (MaxHealth :type "Float (double-precision)"))
  (return 180.0))

(fn `getBuildingType`
  (returns (type :type "/Game/Blueprints/Buildings/BuildingSpotTypes Enum"))
  (return "NewEnumerator1"))

(fn `UserConstructionScript`)