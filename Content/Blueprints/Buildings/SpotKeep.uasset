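; SpotKeep is a clickable building spot for an RTS that accepts a single building type, presumably a keep.
; Clicking its collision area registers it with the RTS_Controller as the current building spot.
; The construction script fills the possible-type list with that one enum entry, which the type getter also returns.
; The current-building getter and build handler are stubs, returning nothing and false.
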(event `self.CollisionArea.OnClicked`
  (params (TouchedComponent :type "PrimitiveComponent Object Reference"))
  (bind _asrts_controller_c (cast `/Game/Blueprints/RTS_Controller` (`GameplayStatics.GetPlayerController` 0)))
  (`/Game/Blueprints/RTS_Controller.Set Current BuildingSpot` _asrts_controller_c self))

(fn `GetBuildingPossibleTypes`
  (returns (NewParam :type "Array of /Game/Blueprints/Buildings/BuildingTypes Enum"))
  (return (`self.buildingtypes`)))

(fn `getBuildingType`
  (returns (type :type "/Game/Blueprints/Buildings/BuildingSpotTypes Enum"))
  (return "NewEnumerator3"))

(fn `GetCurrentBuilding`
  (returns (building :type "/Game/Blueprints/Buildings/Building Object Reference"))
  (return null))

(fn `OnBuildOnSpot`
  (params (BuildingObject :type "/Game/Blueprints/Buildings/BuildingTypes Enum" :default "NewEnumerator0"))
  (returns (state :type Boolean))
  (return false))

(fn `UserConstructionScript`
  (set `self.buildingtypes` (`|MakeArray` "NewEnumerator3" :!type "/Game/Blueprints/Buildings/BuildingTypes Enum")))